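; BP_FinishLine is a finish line actor that counts laps when a BP_ThirdPersonCharacter overlaps it.
; If the character's track progress check passes, it increments LapCount, calls OnLapProgress with it and resets a DoOnce gate.
; A failed check goes through that gate, so it subtracts a lap only once until the next valid crossing.
; Tick prints the current lap count on screen as a debug readout.
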(event `self.ReceiveActorBeginOverlap`
  (params (OtherActor :type "Actor Object Reference"))
  (bind _asbp_third_person_character (cast `/Game/BP_ThirdPersonCharacter` OtherActor))
  (if (`/Game/BP_ThirdPersonCharacter.GetTrackProgress` _asbp_third_person_character)
    (bind _result (`/Engine/EditorBlueprintResources/StandardMacros.IncrementInt` (`self.LapCount`))
      (:`  `
        (`self.OnLapProgress` _result)
        (goto _label :!via `Reset`)))
    (else
      (`/Engine/EditorBlueprintResources/StandardMacros.DoOnce` false :!label _label
        (:`Completed`
          (`/Engine/EditorBlueprintResources/StandardMacros.DecrementInt` (`self.LapCount`)))))))

(event `self.ReceiveTick`
  (params (DeltaSeconds :type "Float (single-precision)"))
  (`KismetSystemLibrary.PrintString` (`KismetStringLibrary.Conv_IntToString` (`self.LapCount`)) true true (struct :`G` 0.66 :`B` 1.0 :`A` 1.0) 0.0))

(fn `UserConstructionScript`)