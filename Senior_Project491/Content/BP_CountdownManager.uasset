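; BP_CountdownManager runs a start countdown after an intro sequence, keeping the player character's input disabled until it finishes.
; On BeginPlay it disables input and binds to the intro sequence player's finished event, which creates the countdown widget and starts a looping one-second timer.
; Each tick decrements the displayed number, then at zero clears the timer, shows "GO!", and after a short delay removes the widget and re-enables input.
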(event `self.ReceiveBeginPlay`
  (`self.DisableInput` (`GameplayStatics.GetPlayerCharacter` 0) (`GameplayStatics.GetPlayerController` 0))
  (add `MovieSceneSequencePlayer.OnFinished` (`LevelSequenceActor.SequencePlayer` (`self.IntroSequenceActor`)) (delegate `StartCountdown`)))

(event `StartCountdown`
  (bind _returnvalue (`|CreateWidget` "/Game/CountdownWidget.CountdownWidget_C"))
  (bind _output_get (set `self.CountdownWidget` _returnvalue))
  (`UserWidget.AddToViewport` _output_get 0)
  (bind _returnvalue_2 (`KismetSystemLibrary.K2_SetTimerDelegate` (delegate `CountdownEvent`) 1.0 true)))

(event `CountdownEvent`
  (`/Engine/EditorBlueprintResources/StandardMacros.DecrementInt` (`self.CountdownValue`)
    (:`  `
      (`TextBlock.SetText` (`/Game/CountdownWidget.CountdownText` (`self.CountdownWidget`)) (`KismetTextLibrary.Conv_IntToText` (`self.CountdownValue`)))
      (if (<= (`self.CountdownValue`) 0)
        (`KismetSystemLibrary.K2_ClearAndInvalidateTimerHandle` (stale `StartCountdown` _returnvalue_2))
        (`TextBlock.SetText` (`/Game/CountdownWidget.CountdownText` (`self.CountdownWidget`)) "GO!")
        (`KismetSystemLibrary.Delay` 1.0)
        (`Widget.RemoveFromParent` (`self.CountdownWidget`))
        (`self.EnableInput` (`GameplayStatics.GetPlayerCharacter` 0) (`GameplayStatics.GetPlayerController` 0))))))

(fn `UserConstructionScript`)